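; BP_Enemy is an enemy pawn that wanders between target points picked at random from its TargetPoints array.
; BeginPlay picks the first target, and Tick picks another at random once the enemy is within the acceptance radius.
; Otherwise, Tick feeds the look-at direction to the target into AddMovementInput, steering straight at it without AI or navmesh pathfinding.
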(event `self.ReceiveBeginPlay`
  (set `self.CurrentTarget` (`|GetArrayItem` (`self.TargetPoints`) (`KismetMathLibrary.RandomInteger` (`KismetArrayLibrary.Array_Length` (`self.TargetPoints`))))))

(event `self.ReceiveTick`
  (params (DeltaSeconds :type "Float (single-precision)"))
  (if (< (`KismetMathLibrary.Vector_Distance` (`self.K2_GetActorLocation`) (`self.K2_GetActorLocation` (`self.CurrentTarget`))) (`self.AcceptanceRaidus`))
    (set `self.CurrentTarget` (`|GetArrayItem` (`self.TargetPoints`) (`KismetMathLibrary.RandomIntegerInRange` 0 (- (`KismetArrayLibrary.Array_Length` (`self.TargetPoints`)) 1))))
    (else
      (`self.AddMovementInput` (`KismetMathLibrary.GetForwardVector` (`KismetMathLibrary.FindLookAtRotation` (`self.K2_GetActorLocation`) (`self.K2_GetActorLocation` (`self.CurrentTarget`))))))))

(fn `UserConstructionScript`)