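; BP_Puerta is a door that reacts to the third-person character entering or leaving its Box trigger.
; Entering sets PlayerDentro and lights every BP_Lampara in the level; leaving clears the flag and zeroes their intensity.
; Entry also starts chained named timers that snap the door down to closed after a delay, then back up to open, without cancelling on exit.
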(event `self.Box.OnComponentEndOverlap`
  (params (OverlappedComponent :type "PrimitiveComponent Object Reference") (OtherActor :type "Actor Object Reference") (OtherComp :type "PrimitiveComponent Object Reference") (OtherBodyIndex :type Integer))
  (cast `/Game/ThirdPerson/Blueprints/BP_ThirdPersonCharacter` OtherActor)
  (set `self.bPlayer Dentro` false)
  (bind _outactors (`GameplayStatics.GetAllActorsOfClass` "/Game/BP/BP_Lampara.BP_Lampara_C"))
  (for _array_element _outactors
    (`LightComponent.SetIntensity` (`/Game/BP/BP_Lampara.PointLight` _array_element) 0.0)))

(event `self.Box.OnComponentBeginOverlap`
  (params (OverlappedComponent :type "PrimitiveComponent Object Reference") (OtherActor :type "Actor Object Reference") (OtherComp :type "PrimitiveComponent Object Reference") (OtherBodyIndex :type Integer) (bFromSweep :type Boolean) (SweepResult :type "HitResult Structure (by ref)"))
  (cast `/Game/ThirdPerson/Blueprints/BP_ThirdPersonCharacter` OtherActor)
  (set `self.bPlayer Dentro` true)
  (bind _outactors (`GameplayStatics.GetAllActorsOfClass` "/Game/BP/BP_Lampara.BP_Lampara_C"))
  (for _array_element _outactors
    (`LightComponent.SetIntensity` (`/Game/BP/BP_Lampara.PointLight` _array_element) 700.0))
  (`KismetSystemLibrary.K2_SetTimer` null "CerrarPuerta" 3.0))

(event `CerrarPuerta`
  (`SceneComponent.K2_SetRelativeLocation` (`self.Puerta`) (-60.0 -101.0 0.0) false false)
  (`KismetSystemLibrary.K2_SetTimer` null "AbrirPuerta" 5.0))

(event `AbrirPuerta`
  (`SceneComponent.K2_SetRelativeLocation` (`self.Puerta`) (-60.0 -101.0 410.0) false false))

(fn `UserConstructionScript`)